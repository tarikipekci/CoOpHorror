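; BP_PlayerCharacter is a player character Blueprint that adds hold-to-crouch and hold-to-sprint controls.
; Holding C crouches unless the character is falling, and releasing it uncrouches.
; Left Shift switches the movement component's MaxWalkSpeed to MaxSpeed while held and to MinSpeed on release.
; Input uses raw key events, and BeginPlay, Tick and the construction script are empty.
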(event `Key|C`
  (params (Key :type "Key Structure"))
  (:`Pressed`
    (if (not (`NavMovementComponent.IsFalling` (`self.CharacterMovement`)))
      (`self.Crouch`)))
  (:`Released`
    (`self.UnCrouch`)))

(event `Key|LeftShift`
  (params (Key :type "Key Structure"))
  (bind _charactermovement (`self.CharacterMovement`))
  (:`Pressed`
    (set `CharacterMovementComponent.MaxWalkSpeed` (`self.MaxSpeed`) _charactermovement))
  (:`Released`
    (set `CharacterMovementComponent.MaxWalkSpeed` (`self.MinSpeed`) _charactermovement)))

(fn `UserConstructionScript`)